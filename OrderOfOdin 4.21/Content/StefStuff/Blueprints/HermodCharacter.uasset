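; Hermod character Blueprint handling aim zoom, projectile firing, footstep sounds, and health with respawn.
; Right mouse or left trigger narrows camera FOV; foot collider overlaps play attached, quietened explosion sounds.
; Left click spawns a projectile from a forward-vector-based transform, also offsetting the character's root.
; Tick adds regeneration without clamping to MaxHealth, or teleports to the stored respawn position and resets health once it drops below zero.
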(event `Key|Gamepad_LeftTrigger`
  (params (Key :type "Key Structure"))
  (bind _followcamera (`self.FollowCamera`))
  ;[1 1 1] Zoom code for aiming
  (:`Pressed`
    (`CameraComponent.SetFieldOfView` _followcamera 60.0 :!label _label))
  (:`Released`
    (`CameraComponent.SetFieldOfView` _followcamera 90.0 :!label _label_2)))

(event `Key|RightMouseButton`
  (params (Key :type "Key Structure"))
  ;[1 1 1] Zoom code for aiming
  (:`Pressed`
    (goto _label))
  (:`Released`
    (goto _label_2)))

(event `self.ReceiveBeginPlay`
  (add `PrimitiveComponent.OnComponentBeginOverlap` (`self.LeftFootCollider`) (delegate `Event LeftFootBeginOverlap`))
  (add `PrimitiveComponent.OnComponentBeginOverlap` (`self.RightFootCollider`) (delegate `Event RightFootBeginOverlap`)))

(event `Event LeftFootBeginOverlap`
  (params (OverlappedComponent :type "PrimitiveComponent Object Reference") (OtherActor :type "Actor Object Reference") (OtherComp :type "PrimitiveComponent Object Reference") (OtherBodyIndex :type Integer) (bFromSweep :type Boolean) (SweepResult :type "HitResult Structure (by ref)"))
  (`GameplayStatics.SpawnSoundAttached` "/Game/StarterContent/Audio/Explosion02.Explosion02" OverlappedComponent "None" (0.0 0.0 0.0) (struct) "KeepRelativeOffset" false 0.2 2.0 0.0 null null))

(event `Event RightFootBeginOverlap`
  (params (OverlappedComponent :type "PrimitiveComponent Object Reference") (OtherActor :type "Actor Object Reference") (OtherComp :type "PrimitiveComponent Object Reference") (OtherBodyIndex :type Integer) (bFromSweep :type Boolean) (SweepResult :type "HitResult Structure (by ref)"))
  (`GameplayStatics.SpawnSoundAttached` "/Game/StarterContent/Audio/Explosion01.Explosion01" OverlappedComponent "None" (0.0 0.0 0.0) (struct) "KeepRelativeOffset" false 0.2 1.0 0.0 null null))

(event `self.ReceiveTick`
  (params (DeltaSeconds :type "Float (single-precision)"))
  (`|ExecutionSequence`
    (:`then_0`
      ;[1 1 1] health regeneration
      (if (< (`self.Health`) 0.0)
        (`self.Respawn`)
        (set `self.Health` 100.0)
        (else
          (`self.RegenHealth`))))))

(event `Key|LeftMouseButton`
  (params (Key :type "Key Structure"))
  (bind _rootcomponent (`self.RootComponent`))
  (bind _returnvalue (+ (`SceneComponent.GetForwardVector` _rootcomponent) 50))
  (:`Pressed`
    (bind _returnvalue_2 (`|SpawnActorFromClass` "/Game/StefStuff/Blueprints/Projectile.Projectile_C" (`KismetMathLibrary.Conv_VectorToTransform` _returnvalue) "Undefined" "OverrideRootScale" null null))
    (`SceneComponent.K2_AddWorldOffset` _rootcomponent _returnvalue false false)
    (`/Game/StefStuff/Blueprints/Projectile.SetupVariables` _returnvalue_2 _returnvalue)))

(fn `ChangeHealth`
  (params (healthChange :type "Float (double-precision)"))
  (bind _output_get (set `self.Health` (+ (`self.Health`) healthChange)))
  (`KismetSystemLibrary.PrintString` (`KismetStringLibrary.Concat_StrStr` "Health is" (`KismetStringLibrary.Conv_DoubleToString` _output_get)) true true (struct :`R` 1.0 :`G` 0.045749 :`A` 1.0)))

(fn `RegenHealth`
  (bind _output_get (set `self.Health` (+ (`self.Health`) (`self.RegenAmount`))))
  (`KismetSystemLibrary.PrintString` (`KismetStringLibrary.Conv_DoubleToString` _output_get) true true (struct :`G` 0.66 :`B` 1.0 :`A` 1.0) 0.1))

(fn `Respawn`
  (`SceneComponent.K2_SetWorldLocation` (`self.CapsuleComponent`) (`self.RespawnPosition`) false false))

(fn `SetRespawnLocation`
  (params (RespawnLocation :type "Vector Structure"))
  (set `self.RespawnPosition` RespawnLocation))

(fn `setupVariables`
  (params (RespawnLocation :type "Vector Structure") (MaxHealth :type "Float (double-precision)") (CurrentHealth :type "Float (double-precision)") (RegenAmount :type "Float (double-precision)") (SelfSceneInstance :type "/Game/StefStuff/Blueprints/HermodCharacter Object Reference"))
  (set `self.RespawnPosition` RespawnLocation)
  (set `self.MaxHealth` MaxHealth)
  (set `self.Health` CurrentHealth)
  (set `self.RegenAmount` RegenAmount)
  (set `self.SelfSceneReference` SelfSceneInstance))

(fn `UserConstructionScript`)