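; FallingRock is an actor that drops a group of eight rocks when the player is inside its trigger volume.
; Tick polls whether the trigger volume overlaps the Player reference, rather than using an overlap event.
; While it does, every rock is set to Movable with gravity enabled, repeated each frame with no one-shot guard.
; GetReferences receives the Player reference from outside.
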(event `self.ReceiveTick`
  (params (DeltaSeconds :type "Float (single-precision)"))
  (bind _rock (`self.Rock`))
  (if (`PrimitiveComponent.IsOverlappingActor` (`self.TriggerVolume`) (`self.Player`))
    (`SceneComponent.SetMobility` _rock "Movable")
    (`SceneComponent.SetMobility` (`self.rock2`) "Movable")
    (`SceneComponent.SetMobility` (`self.rock4`) "Movable")
    (`SceneComponent.SetMobility` (`self.rock5`) "Movable")
    (`SceneComponent.SetMobility` (`self.rock6`) "Movable")
    (`SceneComponent.SetMobility` (`self.rock7`) "Movable")
    (`SceneComponent.SetMobility` (`self.rock8`) "Movable")
    (`SceneComponent.SetMobility` (`self.rock3`) "Movable")
    (`PrimitiveComponent.SetEnableGravity` _rock true)
    (`PrimitiveComponent.SetEnableGravity` (`self.rock2`) true)
    (`PrimitiveComponent.SetEnableGravity` (`self.rock4`) true)
    (`PrimitiveComponent.SetEnableGravity` (`self.rock5`) true)
    (`PrimitiveComponent.SetEnableGravity` (`self.rock6`) true)
    (`PrimitiveComponent.SetEnableGravity` (`self.rock7`) true)
    (`PrimitiveComponent.SetEnableGravity` (`self.rock8`) true)
    (`PrimitiveComponent.SetEnableGravity` (`self.rock3`) true)))

(fn `GetReferences`
  (params (Player :type "/Game/StefStuff/Blueprints/ThirdPersonCharacter Object Reference"))
  (set `self.Player` Player))

(fn `UserConstructionScript`)